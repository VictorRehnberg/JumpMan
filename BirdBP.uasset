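; BirdBP is a flying bird obstacle that kills the player on contact unless they are invisible or ducking.
; From BeginPlay, a delay loop nudges the bird forward along its local X axis in small fixed steps until the player's StopWorld flag is set.
; On overlap with the PlayerBP, it checks the Invis and Ducking flags before calling Death on the player.
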(event `self.ReceiveBeginPlay`
  ;[1 1 1] BeginPlay
  (`self.BirdMovement`))

(event `self.ReceiveActorBeginOverlap`
  (params (OtherActor :type "Actor Object Reference"))
  ;[1 1 1] Collision With Player
  (bind _returnvalue (`GameplayStatics.GetActorOfClass` "/Game/PlayerBP.PlayerBP_C"))
  (if (== OtherActor _returnvalue)
    (if (`/Game/PlayerBP.Invis?` _returnvalue)
      _
      (elif (not (`/Game/PlayerBP.Ducking?` _returnvalue))
        (`/Game/PlayerBP.Death` _returnvalue)))))

(event `BirdMovement`
  ;[1 1 1] Bird
  (`KismetSystemLibrary.Delay` 0.05 :!label _label)
  (`self.K2_AddActorLocalOffset` (10.0 0.0 0.0))
  (bind _returnvalue (`GameplayStatics.GetActorOfClass` "/Game/PlayerBP.PlayerBP_C"))
  (bind _asplayer_bp (cast `/Game/PlayerBP` _returnvalue))
  (if (not (`/Game/PlayerBP.StopWorld?` _asplayer_bp))
    (goto _label)))

(fn `UserConstructionScript`)